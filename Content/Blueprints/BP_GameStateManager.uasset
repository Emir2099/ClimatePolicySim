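; BP_GameStateManager holds four game state metrics: carbon emissions, GDP growth, public support and renewable capacity.
; UpdateVariable adds a change amount to the metric matching a given name, and GetVariableByName returns one by name.
; The two functions expect different name spellings: unspaced variable names for updates, spaced labels for reads, with "Carbon Emission" singular.
; The event graph does nothing, leaving only an unconnected update-and-print test.
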(event EventBeginPlay)

(event Collision|EventActorBeginOverlap
  (params (OtherActor :type Actor%20Object%20Reference)))

(event EventTick
  (params (DeltaSeconds :type Float%20%28single-precision%29)))

(fn ConstructionScript)

(fn UpdateVariable
  (params (VariableName :type String) (ChangeAmount :type Float%20%28double-precision%29))
  (Utilities|FlowControl|Sequence
    (:then_0
      (if (Utilities|Enum|Equal(Enum) VariableName "CarbonEmissions")
        (Variables|Default|SetCarbonEmissions (+ (Variables|Default|GetCarbonEmissions) ChangeAmount))))
    (:then_1
      (if (Utilities|Enum|Equal(Enum) VariableName "GDPGrowth")
        (Variables|Default|SetGDPGrowth (+ (Variables|Default|GetGDPGrowth) ChangeAmount))))
    (:then_2
      (if (Utilities|Enum|Equal(Enum) VariableName "PublicSupport")
        (Variables|Default|SetPublicSupport (+ (Variables|Default|GetPublicSupport) ChangeAmount))))
    (:then_3
      (if (Utilities|Enum|Equal(Enum) VariableName "RenewableCapacity")
        (Variables|Default|SetRenewableCapacity (+ (Variables|Default|GetRenewableCapacity) ChangeAmount))))))

(fn GetVariablebyName
  (params (VariableName :type String))
  (switch string VariableName
    (:CarbonEmission
      (bind _output_get (LocalVariables|SetLocalReturnValue (Variables|Default|GetCarbonEmissions)))
      (return _output_get))
    (:GDPGrowth
      (bind _output_get_2 (LocalVariables|SetLocalReturnValue (Variables|Default|GetGDPGrowth)))
      (return _output_get_2))
    (:PublicSupport
      (bind _output_get_3 (LocalVariables|SetLocalReturnValue (Variables|Default|GetPublicSupport)))
      (return _output_get_3))
    (:RenewableCapacity
      (bind _output_get_4 (LocalVariables|SetLocalReturnValue (Variables|Default|GetRenewableCapacity)))
      (return _output_get_4))))