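; BP_FocusTreeManager is an actor that applies policy decision outcomes to national stats held by BP_GameStateManager.
; ProcessDecisions branches on an option index: option 0 changes carbon emissions and renewable capacity, any other changes GDP growth and public support.
; It finds the manager by class, updates variables by name and prints the new values to screen.
; BeginPlay currently hardcodes option 0, and the decision data variable is unused.
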(event EventBeginPlay
  (CallFunction|ProcessDecisions))

(event Collision|EventActorBeginOverlap
  (params (OtherActor :type Actor%20Object%20Reference)))

(event EventTick
  (params (DeltaSeconds :type Float%20%28single-precision%29)))

(fn ConstructionScript)

(fn ProcessDecisions
  (params (OptionIndex :type Integer))
  (if (== OptionIndex 0)
    (bind _returnvalue (Actor|GetActorOfClass "/Game/Blueprints/BP_GameStateManager.BP_GameStateManager_C"))
    (bind _asbp_game_state_manager (Utilities|Casting|CastToBP_GameStateManager _returnvalue))
    (Default|UpdateVariable _asbp_game_state_manager "CarbonEmissions" 0.5)
    (Default|UpdateVariable _asbp_game_state_manager "RenewableCapacity" 3.0)
    (Development|PrintString (Utilities|String|ToString(Float) (Variables|/Game/Blueprints/BP_GameStateManager.BP_GameStateManager_C|GetCarbonEmissions _asbp_game_state_manager)))
    (Development|PrintString (Utilities|String|ToString(Float) (Variables|/Game/Blueprints/BP_GameStateManager.BP_GameStateManager_C|GetRenewableCapacity _asbp_game_state_manager)))
    (else
      (bind _returnvalue_2 (Actor|GetActorOfClass "/Game/Blueprints/BP_GameStateManager.BP_GameStateManager_C"))
      (bind _asbp_game_state_manager_2 (Utilities|Casting|CastToBP_GameStateManager _returnvalue_2))
      (Default|UpdateVariable _asbp_game_state_manager_2 "GDPGrowth" 1.0)
      (Default|UpdateVariable _asbp_game_state_manager_2 "PublicSupport" -2.0)
      (Development|PrintString (Utilities|String|ToString(Float) (Variables|/Game/Blueprints/BP_GameStateManager.BP_GameStateManager_C|GetGDPGrowth _asbp_game_state_manager_2)))
      (Development|PrintString (Utilities|String|ToString(Float) (Variables|/Game/Blueprints/BP_GameStateManager.BP_GameStateManager_C|GetPublicSupport _asbp_game_state_manager_2))))))